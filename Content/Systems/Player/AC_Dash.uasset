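; AC_Dash is a player dash component for BP_Player, which it caches with its CharacterMovement on Initialize.
; Dash makes one swept VInterpTo step per call toward the GetDashDirection endpoint, using wish direction and Data speed.
; Landing or ending a grapple re-enables CanDash, though Dash never checks it.
; GetDashDirection is unfinished: its distance-along-direction calculation is left unconnected.
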(event Custom|Initialize
  (bind _asbp_player (Utilities|Casting|CastToBP_Player (Components|GetOwner)))
  (bind _output_get (Variables|Default|Setplayer _asbp_player))
  (Variables|Default|SetCharacter%20Movement (Variables|/Script/Engine.Character|GetCharacterMovement _output_get)))

(event Custom|OnLand
  (Variables|Default|SetCanDash true))

(event Custom|OnGrappleEnd
  (Variables|Default|SetCanDash true))

(fn Dash
  (bind _newparam (Default|GetWishDirection (Variables|Default|Getplayer)))
  (Transformation|SetActorLocation (Variables|Default|Getplayer) (Math|Interpolation|VInterpTo (Transformation|GetActorLocation (Variables|Default|Getplayer)) (.endPoint (Utilities|GetDashDirection _newparam)) (Utilities|Time|GetWorldDeltaSeconds) (Variables|/Game/Systems/Player/PDA_Dash.PDA_Dash_C|GetSpeed (Variables|Default|Getdata))) true false))