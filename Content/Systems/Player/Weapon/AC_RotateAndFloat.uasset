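; Actor component in the player weapon systems, named for rotating and floating its owning actor.
; It stores the owner's location on BeginPlay and calls SetActorLocationAndRotation on the owner every Tick.
; GetFloatPosition holds a sine-over-time bob around the starting height, scaled by FloatDeviation, but it appears unused.
; The Tick call shows no location or rotation inputs.
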(event EventBeginPlay
  (Variables|Default|SetStartPosition (Transformation|GetActorLocation (Components|GetOwner))))

(event EventTick
  (params (DeltaSeconds :type Float%20%28single-precision%29))
  (Transformation|SetActorLocationAndRotation (Components|GetOwner) (Math|Vector|MakeVector 0.0 0.0 0.0)))