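; AC_Float is an actor component that bobs its owner in place, apparently for weapon objects under the player systems.
; On BeginPlay it caches the owner's location, then each Tick sets the location to a float position or back to that start point, depending on the Float flag.
; GetFloatPosition holds an unconnected time-based sine height offset, and GetRotation is empty.
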(event EventBeginPlay
  (Variables|Default|SetStartPosition (Transformation|GetActorLocation (Components|GetOwner))))

(event EventTick
  (params (DeltaSeconds :type Float%20%28single-precision%29))
  (Transformation|SetActorLocation (Components|GetOwner) (select (Variables|Default|GetFloat) (Utilities|GetFloatPosition) (Variables|Default|GetStartPosition)) false false))