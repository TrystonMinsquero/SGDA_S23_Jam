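; Player actor component that adds wall running, gated by an ability on BP_Player.
; A looping timer traces right and left while the player moves forward, and on airborne hits against Wall physical material uses LaunchCharacter along the surface while easing gravity.
; Ending a run restores gravity, jump count and dash, then briefly suppresses re-attachment.
; Tick eases camera roll by wall side, and WallRunJump launches the player along the wall normal.
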(event Custom|Initialize
  (bind _asbp_player (Utilities|Casting|CastToBP_Player (Components|GetOwner)))
  (bind _output_get (Variables|Default|Setplayer _asbp_player))
  (bind _output_get_2 (Variables|Default|SetCharacterMovement (Variables|/Script/Engine.Character|GetCharacterMovement _output_get)))
  (Variables|Default|SetdefaultGravity (Variables|/Script/Engine.CharacterMovementComponent|GetGravityScale _output_get_2))
  (Utilities|Time|SetTimerbyEvent (delegate Custom|WallRunUpdateEvent) 0.02 true))

(event Custom|WallRunUpdateEvent
  (if (not (Variables|Default|GetwallRunSuppressed))
    (CallFunction|WallRunUpdate)))

(event Custom|ResetWallRunSuppression
  (Utilities|Time|ClearTimerbyFunctionName 0 "ResetWallRunSuppression")
  (Variables|Default|SetwallRunSuppressed false))

(event Custom|OnLand
  (CallFunction|WallRunEnd 0.0)
  (Variables|Default|SetwallRunSuppressed false))

(event EventTick
  (params (DeltaSeconds :type Float%20%28single-precision%29))
  (CallFunction|CameraTick))

(fn WallRunMovement
  (params (Start :type Vector) (End :type Vector) (WallRunDirection :type Float%20%28double-precision%29))
  (bind _outhit (Collision|LineTraceByChannel Start End "TraceTypeQuery1" false 0 "None"))
  (if (.bblockinghit _outhit)
    (if (Math|Boolean|ANDBoolean (AI|Components|NavMovement|IsFalling (Variables|/Script/Engine.Character|GetCharacterMovement (Variables|Default|Getplayer))) true (== (.physmat _outhit) "/Game/Systems/Environment/Wall.Wall"))
      (bind _output_get (Variables|Default|SetWallRunNormal (.normal _outhit)))
      (Character|LaunchCharacter (Variables|Default|Getplayer) (Utilities|PlayertoWallVector _output_get) false false) ; Stick To Wall
      (Character|LaunchCharacter (Variables|Default|Getplayer) (* (Math|Vector|CrossProduct _output_get "0.000000,0.000000,1.000000") (* (Variables|/Game/Systems/Player/PDA_WallRun.PDA_WallRun_C|GetWallRunSpeed (Variables|Default|Getdata)) WallRunDirection)) true (not (Variables|/Game/Systems/Player/PDA_WallRun.PDA_WallRun_C|GetUsesGravity (Variables|Default|Getdata)))) ; Move Speed
      (return true)
      (else
        _)))
  (return false))

(fn WallRunUpdate
  (bind (_right _left) (Utilities|GetEndPoints))
  (bind _data (Variables|Default|Getdata))
  (if (Utilities|Set|Contains (Variables|/Game/Systems/Player/BP_Player.BP_Player_C|Getabilities (Variables|Default|Getplayer)) "NewEnumerator1")
    (bind _returnvalue (Default|GetMoveDirection (Variables|Default|Getplayer)))
    (if (> (.y _returnvalue) 0.0)
      (bind _onwall (CallFunction|WallRunMovement (Transformation|GetActorLocation (Variables|Default|Getplayer)) _right -1.0))
      (if _onwall
        (Variables|Default|SetWallRunningR true)
        (Variables|Default|SetWallRunningL false)
        (Variables|/Script/Engine.CharacterMovementComponent|SetGravityScale (Variables|Default|GetCharacterMovement) (Math|Interpolation|FInterpTo (Variables|/Script/Engine.CharacterMovementComponent|GetGravityScale (Variables|Default|GetCharacterMovement)) (Variables|/Game/Systems/Player/PDA_WallRun.PDA_WallRun_C|GetWallRunTargetGravity _data) (Utilities|Time|GetWorldDeltaSeconds) (Variables|/Game/Systems/Player/PDA_WallRun.PDA_WallRun_C|GetGravityLerpSpeed _data)) :!label _label)
        (elif (Variables|Default|GetWallRunningR)
          (CallFunction|WallRunEnd (Variables|/Game/Systems/Player/PDA_WallRun.PDA_WallRun_C|GetResetTimeAfterFall (Variables|Default|Getdata)))
          (else
            (bind _onwall_2 (CallFunction|WallRunMovement (Transformation|GetActorLocation (Variables|Default|Getplayer)) _left 1.0))
            (if _onwall_2
              (Variables|Default|SetWallRunningR false)
              (Variables|Default|SetWallRunningL true)
              (goto _label)
              (else
                (CallFunction|WallRunEnd (Variables|/Game/Systems/Player/PDA_WallRun.PDA_WallRun_C|GetResetTimeAfterFall (Variables|Default|Getdata))))))))
      (else
        (CallFunction|WallRunEnd (Variables|/Game/Systems/Player/PDA_WallRun.PDA_WallRun_C|GetResetTimeAfterFall (Variables|Default|Getdata)))))))

(fn WallRunEnd
  (params (ResetTime :type Float%20%28double-precision%29))
  (if (or (Variables|Default|GetWallRunningR) (Variables|Default|GetWallRunningL))
    (Variables|Default|SetWallRunningR false)
    (Variables|Default|SetWallRunningL false)
    (Variables|/Game/Systems/Player/BP_Player.BP_Player_C|SetjumpCounter (Variables|Default|Getplayer) 1)
    (Variables|/Game/Systems/Player/BP_Player.BP_Player_C|SetbCanDash (Variables|Default|Getplayer) true)
    (Variables|/Script/Engine.CharacterMovementComponent|SetGravityScale (Variables|Default|GetCharacterMovement) (Variables|Default|GetdefaultGravity))
    (CallFunction|SuppressWallRun ResetTime)))

(fn SuppressWallRun
  (params (delay :type Float%20%28double-precision%29))
  (Variables|Default|SetwallRunSuppressed true)
  (Utilities|Time|SetTimerbyFunctionName 0 "ResetWallRunSuppression" delay))

(fn CameraTick
  (bind _data (Variables|Default|Getdata))
  (bind _camera_tilt (Variables|/Game/Systems/Player/PDA_WallRun.PDA_WallRun_C|GetCamera%20Tilt _data))
  (if (Variables|Default|GetWallRunningL)
    (CallFunction|CameraTilt _camera_tilt)
    (elif (Variables|Default|GetWallRunningR)
      (CallFunction|CameraTilt (* _camera_tilt -1.0))
      (else
        (CallFunction|CameraTilt 0.0)))))

(fn CameraTilt
  (params (Target%20Roll%20%28X%29 :type Float%20%28double-precision%29))
  (bind _player (Variables|Default|Getplayer))
  (bind _returnvalue (Pawn|GetController _player))
  (bind _returnvalue_2 (Pawn|GetControlRotation _returnvalue :!class /Script/Engine.Controller))
  (bind (_roll _pitch _yaw) (Math|Rotator|BreakRotator _returnvalue_2))
  (Pawn|SetControlRotation (Pawn|GetController (Variables|Default|Getplayer)) (Math|Interpolation|RInterpTo _returnvalue_2 (Math|Rotator|MakeRotator Target%20Roll%20%28X%29 _pitch _yaw) (Utilities|Time|GetWorldDeltaSeconds) (Variables|/Game/Systems/Player/PDA_WallRun.PDA_WallRun_C|GetCameraTiltLerpSpeed (Variables|Default|Getdata)))))

(fn WallRunJump
  (bind _data (Variables|Default|Getdata))
  (bind _wallrunnormal (Variables|Default|GetWallRunNormal))
  (bind _jumpforce (Variables|/Game/Systems/Player/PDA_WallRun.PDA_WallRun_C|GetJumpForce _data))
  (if (or (Variables|Default|GetWallRunningR) (Variables|Default|GetWallRunningL))
    (CallFunction|WallRunEnd (Variables|/Game/Systems/Player/PDA_WallRun.PDA_WallRun_C|GetResetTimeAfterJump (Variables|Default|Getdata)))
    (Character|LaunchCharacter (Variables|Default|Getplayer) (Math|Vector|MakeVector (* _jumpforce (.x _wallrunnormal)) (* _jumpforce (.y _wallrunnormal)) (Variables|/Game/Systems/Player/PDA_WallRun.PDA_WallRun_C|GetJumpHeight (Variables|Default|Getdata))) false false)
    (return true)
    (else
      (return false))))

(fn OnJump
  (CallFunction|WallRunJump))