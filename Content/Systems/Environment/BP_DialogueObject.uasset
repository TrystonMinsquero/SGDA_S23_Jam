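; BP_DialogueObject is an interactable object that shows dialogue lines to the player, one per Interact call.
; On BeginPlay it creates the dialogue widget and caches BP_Player's movement component.
; ShowNextLine freezes movement on the first line, advances an index, then removes the widget, restores walking and sets Finished after the last line.
; Interact plays EndLines until Finished is set, then StartLines, an order the variable names suggest is reversed.
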(event EventBeginPlay
  (bind _returnvalue (UserInterface|CreateWidget "/Game/UI/WBP_Diaglogue.WBP_Diaglogue_C" (Game|GetPlayerController 0)))
  (Variables|Default|SetdiaglogueWidget _returnvalue)
  (bind _asbp_player (Utilities|Casting|CastToBP_Player (Game|Player|GetPlayerPawn 0)))
  (Variables|Default|SetCharacter%20Movement (Variables|/Script/Engine.Character|GetCharacterMovement _asbp_player)))

(event EventInteract
  (params (Player :type BP%20Player%20Object%20Reference))
  (if (Variables|Default|Getfinished)
    (CallFunction|ShowNextLine (Variables|Default|GetstartLines))
    (else
      (CallFunction|ShowNextLine (Variables|Default|GetendLines)))))

(fn ConstructionScript)

(fn ShowNextLine
  (params (lines :type Array%20of%20Texts))
  (if (== 0 (Variables|Default|Getindex))
    (Pawn|Components|CharacterMovement|DisableMovement (Variables|Default|GetCharacter%20Movement))
    (UserInterface|Viewport|AddtoViewport (Variables|Default|GetdiaglogueWidget) 0)
    (Default|UpdateText (Variables|Default|GetdiaglogueWidget) (Utilities|Array|Get(acopy) lines (Variables|Default|Getindex)) :!label _label)
    (Math|Integer|IncrementInt (Variables|Default|Getindex))
    (elif (< (Variables|Default|Getindex) (Utilities|Array|Length lines))
      (goto _label)
      (else
        (Widget|RemovefromParent (Variables|Default|GetdiaglogueWidget))
        (Pawn|Components|CharacterMovement|SetMovementMode (Variables|Default|GetCharacter%20Movement) "MOVE_Walking" 0)
        (Variables|Default|Setfinished true)
        (Variables|Default|Setindex 0)))))