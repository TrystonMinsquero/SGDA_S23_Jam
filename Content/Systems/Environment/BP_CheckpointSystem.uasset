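; BP_CheckpointSystem is a level checkpoint manager that tracks player progress and handles respawning.
; On BeginPlay it binds to each checkpoint's entered event and to the player's death event, then teleports the player to the current point.
; Entering a checkpoint raises the current index to its array position, never lowering it, so array order defines progression.
; Death teleports the player to that checkpoint's location and rotation.
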(event Custom|OnEnterCheckpoint
  (params (checkpoint :type BP%20Checkpoint%20Object%20Reference))
  (Variables|Default|SetcurrentPoint (Math|Integer|Max(Integer) (Utilities|Array|FindItem (Variables|Default|Getcheckpoints) checkpoint) (Variables|Default|GetcurrentPoint))))

(event Custom|SetPlayerToCurrentPoint
  (bind _currentpoint (Variables|Default|GetcurrentPoint))
  (bind _checkpoints (Variables|Default|Getcheckpoints))
  (bind _output (Utilities|Array|Get(acopy) _checkpoints _currentpoint))
  (Transformation|SetActorLocationAndRotation (Game|Player|GetPlayerPawn 0) (Transformation|GetActorLocation _output) (Transformation|GetActorRotation _output) false true))

(event EventBeginPlay
  (for _array_element (Variables|Default|Getcheckpoints)
    (EventDispatchers|BindEventtoPlayerEnteredCheckpoint _array_element (delegate Custom|OnEnterCheckpoint)))
  (CallFunction|SetPlayertoCurrentPoint)
  (bind _asbp_player (Utilities|Casting|CastToBP_Player (Game|Player|GetPlayerPawn 0)))
  (EventDispatchers|BindEventtoDied _asbp_player (delegate Custom|SetPlayerToCurrentPoint)))

(fn ConstructionScript)