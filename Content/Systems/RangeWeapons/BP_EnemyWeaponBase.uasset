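; BP_EnemyWeaponBase is a base ranged weapon for enemies that fires bullets at the player.
; On begin play it casts and stores its BP_BaseEnemy owner.
; StartShooting and StopShooting toggle a looping timer at the data's fire rate, which calls FireBullet.
; FireBullet spawns the data's bullet type at the enemy's fire position, rotated toward the player pawn's current location.
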(event Custom|StartShooting
  (if (not (Variables|Default|GetIsShooting))
    (Variables|Default|SetIsShooting true)
    (bind _returnvalue (Utilities|Time|SetTimerbyFunctionName 0 "FireBullet" (Variables|/Game/Systems/RangeWeapons/PDA_EnemyWeaponData.PDA_EnemyWeaponData_C|GetFireRate (Variables|Default|Getdata)) true))
    (Variables|Default|Settimer _returnvalue)))

(event Custom|StopShooting
  (if (Variables|Default|GetIsShooting)
    (Variables|Default|SetIsShooting false)
    (Utilities|Time|ClearandInvalidateTimerbyHandle (Variables|Default|Gettimer))))

(event EventBeginPlay
  (bind _asbp_base_enemy (Utilities|Casting|CastToBP_BaseEnemy (Components|GetOwner)))
  (Variables|Default|SetEnemy _asbp_base_enemy))

(fn FireBullet
  (bind _returnvalue (Default|GetFirePosition (Variables|Default|GetEnemy)))
  (Game|SpawnActorfromClass (Variables|/Game/Systems/RangeWeapons/PDA_EnemyWeaponData.PDA_EnemyWeaponData_C|GetBulletType (Variables|Default|Getdata)) (Math|Transform|MakeTransform _returnvalue (Math|Rotator|FindLookatRotation _returnvalue (Transformation|GetActorLocation (Game|Player|GetPlayerPawn 0))) "1.000000,1.000000,1.000000") "Undefined" 0 0))