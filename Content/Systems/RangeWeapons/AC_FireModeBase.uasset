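; Base actor component for enemy ranged fire modes, holding the shared shooting state and bullet-firing logic.
; On BeginPlay it caches the owning BP_BaseEnemy.
; FireBullet spawns the data-defined bullet class at the enemy's fire position, rotated toward the player pawn, and plays the fire montage.
; Start and stop functions toggle IsShooting and return whether the state changed.
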(event EventBeginPlay
  (bind _asbp_base_enemy (Utilities|Casting|CastToBP_BaseEnemy (Components|GetOwner)))
  (Variables|Default|SetEnemy _asbp_base_enemy))

(fn FireBullet
  (bind _returnvalue (Default|GetFirePosition (Variables|Default|GetEnemy)))
  (Game|SpawnActorfromClass (Variables|/Game/Systems/RangeWeapons/PDA_EnemyWeaponData.PDA_EnemyWeaponData_C|GetBulletType (Variables|Default|Getdata)) (Math|Transform|MakeTransform _returnvalue (Math|Rotator|FindLookatRotation _returnvalue (Transformation|GetActorLocation (Game|Player|GetPlayerPawn 0))) "1.000000,1.000000,1.000000") "Undefined" 0 0)
  (Default|PlayEnemyAnimMontage (Variables|Default|GetEnemy) (Variables|Default|GetFireMontage)))

(fn StartShootingMode
  (if (Variables|Default|GetIsShooting)
    (return false)
    (else
      (Variables|Default|SetIsShooting true)
      (return true))))

(fn StopShooting
  (if (Variables|Default|GetIsShooting)
    (Variables|Default|SetIsShooting false)
    (return true)
    (else
      (return false))))