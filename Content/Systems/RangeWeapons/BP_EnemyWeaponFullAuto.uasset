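; Enemy full-auto ranged weapon Blueprint that fires bullets continuously while shooting is active.
; StartShooting calls the parent logic, then starts a looping timer that calls FireBullet at the fire rate from its weapon data.
; StopShooting calls the parent logic and clears that timer.
; Both events check IsShooting so repeated start or stop calls are ignored.
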(event EventStartShooting
  (if (not (Variables|Default|GetIsShooting))
    (|CallParentFunction)
    (bind _returnvalue (Utilities|Time|SetTimerbyFunctionName 0 "FireBullet" (Variables|/Game/Systems/RangeWeapons/PDA_EnemyWeaponData.PDA_EnemyWeaponData_C|GetFireRate (Variables|Default|Getdata)) true))
    (Variables|Default|SetTimer_0 _returnvalue)))

(event EventStopShooting
  (if (Variables|Default|GetIsShooting)
    (|CallParentFunction)
    (Utilities|Time|ClearandInvalidateTimerbyHandle (Variables|Default|GetTimer_0))))