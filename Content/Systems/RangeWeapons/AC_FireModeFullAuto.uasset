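; AC_FireModeFullAuto is a fire mode component for ranged weapons that provides full-auto shooting.
; When the parent StartShootingMode succeeds, it starts a looping timer that calls FireBullet at the fire rate from the weapon data.
; When the parent StopShooting succeeds, it clears that timer and returns true, otherwise false.
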(fn StartShootingMode
  (bind _changed (|CallParentFunction))
  (if _changed
    (bind _returnvalue (Utilities|Time|SetTimerbyFunctionName 0 "FireBullet" (Variables|/Game/Systems/RangeWeapons/PDA_EnemyWeaponData.PDA_EnemyWeaponData_C|GetFireRate (Variables|Default|Getdata)) true))
    (Variables|Default|SetTimer_0 _returnvalue)))

(fn StopShooting
  (bind _changed (|CallParentFunction))
  (if _changed
    (Utilities|Time|ClearandInvalidateTimerbyHandle (Variables|Default|GetTimer_0))
    (return true)
    (else
      (return false))))