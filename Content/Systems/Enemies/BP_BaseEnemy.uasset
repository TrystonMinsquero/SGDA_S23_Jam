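; Base enemy character with stats from a Data asset, reacting to hits, grapples and player sightings; death only prints a message.
; Damage, sight and grappling set blackboard flags for its AI.
; Point hits juggle it when airborne until a combo count triggers multiplied damage, knockback and stun.
; Stun shows a text indicator and clears on landing, or after a post-grapple delay if grounded.
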(event OnSeePawn(PawnSensing)
  (params (Pawn :type Pawn%20Object%20Reference))
  (bind _returnvalue (Utilities|GetBlackboard))
  (Utilities|Casting|CastToBP_Player Pawn)
  (AI|Components|Blackboard|SetValueasBool _returnvalue (Variables|Default|GetnSeesPlayer) true)
  (AI|Components|Blackboard|SetValueasBool _returnvalue (Variables|Default|GetnIsAggro) true))

(event Custom|OnTakePointDamage_Event
  (params (DamagedActor :type Actor%20Object%20Reference) (Damage :type Float%20%28single-precision%29) (InstigatedBy :type Controller%20Object%20Reference) (HitLocation :type Vector) (FHitComponent :type Primitive%20Component%20Object%20Reference) (BoneName :type Name) (ShotFromDirection :type Vector) (DamageType :type Damage%20Type%20Object%20Reference) (DamageCauser :type Actor%20Object%20Reference))
  (AI|Components|Blackboard|SetValueasBool (Utilities|GetBlackboard) (Variables|Default|GetnIsAggro) true)
  (bind _result (Math|Integer|IncrementInt (Variables|Default|GethitCounter))
    (:%20%20
      (if (>= _result (Variables|/Game/Systems/Enemies/PDA_EnemyData.PDA_EnemyData_C|GetComboCount (Variables|Default|Getdata)))
        (CallFunction|TakeDamage (* Damage (Variables|/Game/Systems/Enemies/PDA_EnemyData.PDA_EnemyData_C|GetComboDamageMultiplier (Variables|Default|Getdata))))
        (Variables|Default|SethitCounter 0)
        (CallFunction|Knockback (Transformation|GetActorLocation DamageCauser))
        (CallFunction|SetStunned true)
        (else
          (CallFunction|TakeDamage Damage)
          (CallFunction|Juggle))))))

(event Custom|Stun
  (params (duration :type Float%20%28double-precision%29))
  (CallFunction|SetStunned true)
  (Utilities|FlowControl|Delay duration)
  (if (AI|Components|NavMovement|IsMovingonGround (Variables|Character|GetCharacterMovement))
    (CallFunction|SetStunned false)))

(event EventBeginPlay
  (bind _charactermovement (Variables|Character|GetCharacterMovement))
  (bind _data (Variables|Default|Getdata))
  (Variables|Default|Sethealth (Variables|/Game/Systems/Enemies/PDA_EnemyData.PDA_EnemyData_C|GetMaxHealth (Variables|Default|Getdata)))
  (EventDispatchers|BindEventtoOnTakePointDamage (delegate Custom|OnTakePointDamage_Event))
  (Variables|/Script/Engine.CharacterMovementComponent|SetMaxWalkSpeed _charactermovement (Variables|/Game/Systems/Enemies/PDA_EnemyData.PDA_EnemyData_C|GetMoveSpeed _data))
  (Variables|/Script/Engine.CharacterMovementComponent|SetGravityScale _charactermovement (Variables|/Game/Systems/Enemies/PDA_EnemyData.PDA_EnemyData_C|GetGravityScale _data)))

(event EventOnLanded
  (params (Hit :type Hit%20Result%20Structure%20%28by%20ref%29))
  (CallFunction|SetStunned false))

(fn ConstructionScript)

(fn TakeDamage
  (params (damage :type Float%20%28double-precision%29))
  (bind _output_get (Variables|Default|Sethealth (- (Variables|Default|Gethealth) damage)))
  (if (<= _output_get 0.0)
    (Development|PrintString "Die!")))

(fn Knockback
  (params (knockbackSourceVector :type Vector))
  (bind _returnvalue (Transformation|GetActorLocation))
  (bind _data (Variables|Default|Getdata))
  (bind _returnvalue_2 (Math|Vector|GetUnitDirection(Vector) knockbackSourceVector _returnvalue))
  (bind _knockbackamount (Variables|/Game/Systems/Enemies/PDA_EnemyData.PDA_EnemyData_C|GetKnockbackAmount _data))
  (bind _returnvalue_3 (* _returnvalue_2 _knockbackamount))
  (if (Variables|/Game/Systems/Enemies/PDA_EnemyData.PDA_EnemyData_C|GetCanKnockback (Variables|Default|Getdata))
    (Components|Movement|StopMovementImmediately (Variables|Character|GetCharacterMovement))
    (Character|LaunchCharacter (Math|Vector|MakeVector (.x _returnvalue_3) (.y _returnvalue_3) (Variables|/Game/Systems/Enemies/PDA_EnemyData.PDA_EnemyData_C|GetKnockbackHeight _data)) true true)))

(fn SetGrappled
  (params (value :type Boolean))
  (bind _self self)
  (bind _returnvalue (AI|GetAIController _self))
  (bind _returnvalue_2 (AI|GetBlackboard _returnvalue))
  (AI|Components|Blackboard|SetValueasBool _returnvalue_2 (Variables|Default|GetnIsGrappled) value)
  (if value
    (AI|Components|Blackboard|SetValueasBool _returnvalue_2 (Variables|Default|GetnIsAggro) true)
    (Class|NavMovementComponent|StopActiveMovement (Variables|Character|GetCharacterMovement))
    (else
      (CallFunction|Stun (Variables|/Game/Systems/Enemies/PDA_EnemyData.PDA_EnemyData_C|GetStunTimeAfterGrapple (Variables|Default|Getdata))))))

(fn GetFirePosition
  (return (Transformation|GetWorldLocation (Variables|Default|GetFirePoint))))

(fn Juggle
  (bind _charactermovement (Variables|Character|GetCharacterMovement))
  (if (and (Variables|/Game/Systems/Enemies/PDA_EnemyData.PDA_EnemyData_C|GetCanJuggle (Variables|Default|Getdata)) (not (AI|Components|NavMovement|IsMovingonGround _charactermovement)))
    (Character|LaunchCharacter (Math|Vector|MakeVector 0.0 0.0 (Variables|/Game/Systems/Enemies/PDA_EnemyData.PDA_EnemyData_C|GetJuggleHeight (Variables|Default|Getdata))) false (< (.z (Variables|/Script/Engine.MovementComponent|GetVelocity _charactermovement)) 0.0))))

(fn SetStunned
  (params (value :type Boolean))
  (AI|Components|Blackboard|SetValueasBool (Utilities|GetBlackboard) (Variables|Default|GetnStunned) value)
  (Rendering|SetVisibility (Variables|Default|GetStunText) value false))

(fn GetGrapplePoint
  (return (Transformation|GetWorldLocation (Variables|Default|GetGrapplePoint))))